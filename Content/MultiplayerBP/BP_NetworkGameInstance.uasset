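; Game instance Blueprint that hosts and joins multiplayer sessions and reports network failures.
; CreateGame creates a 16-slot LAN session, then opens Level1 as a listen server.
; JoinToGame joins the search result held in GameSession, which is not populated in this graph.
; Session, network and travel failures are only printed to screen, with no recovery logic.
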(event Custom|CreateGame
  ;[1 1 1] Create Game Event
  (|Session (Game|GetPlayerController 0) 16 true
    (:OnSuccess
      (Game|OpenLevel(byName) "Level1" true "listen"))
    (:OnFailure
      (Development|PrintString "Game creation error!"))))

(event Custom|JoinToGame
  ;[1 1 1] Join session
  (|JoinSession (Game|GetPlayerController 0) (Variables|Default|GetGameSession)
    (:OnFailure
      (Development|PrintString "Join to game error!"))))

(event EventHandleNetworkError
  (params (FailureType :type ENetworkFailure%20Enum :default "NetDriverAlreadyExists") (bIsServer :type Boolean))
  ;[1 1 1] Network Error
  (Development|PrintString (Utilities|String|Append "Network error:" (Utilities|String|EnumtoString FailureType) "on server?" (Utilities|String|ToString(Boolean) bIsServer))))

(event EventHandleTravelError
  (params (FailureType :type ETravelFailure%20Enum :default "NoLevel"))
  ;[1 1 1] Travel Error
  (Development|PrintString (Utilities|String|Append "Network travel error:" (Utilities|String|EnumtoString FailureType))))