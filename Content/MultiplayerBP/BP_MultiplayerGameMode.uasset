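; Multiplayer game mode that sorts joining players into two teams to keep team sizes balanced.
; On PostLogin it casts the new controller to BP_MultiplayerPlayerController, sets its team ID and adds it to the Team1 or Team2 array.
; Team 2 receives the player only when Team 1 is larger, so ties go to Team 1.
; The logout event is empty, so departing players are not removed from the arrays here.
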(event EventBeginPlay)

(event EventTick
  (params (DeltaSeconds :type Float%20%28single-precision%29)))

(event EventPostLogin
  (params (NewPlayer :type Player%20Controller%20Object%20Reference))
  ;[1 1 1] Set Team
  (bind _asbp_multiplayer_player_controller (Utilities|Casting|CastToBP_MultiplayerPlayerController NewPlayer)
    (:then
      (if (> (Utilities|Array|Length (Variables|Default|GetTeam1)) (Utilities|Array|Length (Variables|Default|GetTeam2)))
        (Default|SetTeamID _asbp_multiplayer_player_controller 2)
        (Utilities|Array|Add (Variables|Default|GetTeam2) _asbp_multiplayer_player_controller)
        (else
          (Default|SetTeamID _asbp_multiplayer_player_controller 1)
          (Utilities|Array|Add (Variables|Default|GetTeam1) _asbp_multiplayer_player_controller))))
    (:CastFailed
      (Development|PrintString "Post login error"))))

(event EventOnLogout
  (params (ExitingController :type Controller%20Object%20Reference)))

(fn ConstructionScript)