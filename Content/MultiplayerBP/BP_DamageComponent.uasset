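; Multiplayer damage component that tracks Health and shows it on a health bar widget.
; TakeDamage forwards the damage value to a server event, which subtracts it from Health with no clamping or death handling.
; OnRep_Health casts the stored widget to WBP_HealthBar and sets its progress bar to Health as a fraction of a hardcoded maximum of 10.
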(event Custom|TakeDamage
  (params (DamageValue :type Float%20%28single-precision%29))
  ;[1 1 1] TakeDamage calls out
  (CallFunction|ServerTakeDamage DamageValue))

(event Custom|Server_TakeDamage
  (params (DamageValue :type Float%20%28single-precision%29))
  ;[1 1 1] TakeDamage Event
  (Variables|Default|SetHealth (- (Variables|Default|GetHealth) DamageValue)))

(event EventBeginPlay)

(event EventTick
  (params (DeltaSeconds :type Float%20%28single-precision%29)))

(fn OnRepHealth
  (bind _asbpw_health_bar (Utilities|Casting|CastToWBP_HealthBar (Variables|Default|GetWidgetHealthBar)))
  (Progress|SetPercent (Variables|/Game/WBP_HealthBar.WBP_HealthBar_C|GetProgressBar_56 _asbpw_health_bar) (/ (Variables|Default|GetHealth) 1e+01)))