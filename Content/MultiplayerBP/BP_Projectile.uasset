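; Multiplayer projectile Blueprint that flies forward, damages pawns on contact and explodes, with gameplay driven by the server.
; The server moves it each Tick without sweep and handles sphere overlaps, ignoring the owner, other projectiles and repeat hits.
; A valid hit damages any BP_MultiplayerPawn through its damage component and multicasts the explosion effect.
; A hit or lifetime timer hides the actor, then destroys it after a short delay.
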(event OnComponentBeginOverlap(Sphere)
  (params (OverlappedComponent :type Primitive%20Component%20Object%20Reference) (OtherActor :type Actor%20Object%20Reference) (OtherComp :type Primitive%20Component%20Object%20Reference) (OtherBodyIndex :type Integer) (bFromSweep :type Boolean) (SweepResult :type Hit%20Result%20Structure%20%28by%20ref%29))
  ;[1 1 1] Collision call on overlap
  (if (Networking|IsServer)
    (CallFunction|ServerCollision OtherActor (Transformation|GetActorLocation))))

(event Custom|Life%20Ended
  ;[1 1 1] Destroy On Time
  (CallFunction|ServerLIfeEnded))

(event Custom|Server_LIfeEnded
  ;[1 1 1] Destroy On Time
  (Rendering|SetActorHiddenInGame true)
  (Utilities|FlowControl|Delay 0.2)
  (Actor|DestroyActor))

(event Custom|SpawnHitEffects
  (params (HitLocation :type Vector))
  ;[1 1 1] HitEffects Spawn
  (Effects|SpawnEmitteratLocation "/Game/StarterContent/Particles/P_Explosion.P_Explosion" HitLocation))

(event Custom|Milticast_HitEffects
  (params (HitLocation :type Vector))
  ;[1 1 1] HitEffects Spawn
  (CallFunction|SpawnHitEffects HitLocation))

(event Custom|Server_Move
  (params (DeltaTime :type Float%20%28single-precision%29))
  ;[1 1 1] Move Event
  (Transformation|SetActorLocation (+ (Transformation|GetActorLocation) (* (Transformation|GetActorForwardVector) (* DeltaTime (Variables|Default|GetSpeed)))) false false))

(event Custom|Server_Collision
  (params (OtherActor :type Actor%20Object%20Reference) (Location :type Vector))
  ;[1 1 1] Collision event Replicated
  (if (and (!= (Components|GetOwner) OtherActor) (not (Variables|Default|GetbCollided)))
    (bind _asbp_multiplayer_pawn (Utilities|Casting|CastToBP_MultiplayerPawn OtherActor)
      (:then
        (Default|TakeDamage (Variables|/Game/MultiplayerBP/BP_MultiplayerPawn.BP_MultiplayerPawn_C|GetBP_DamageComponent _asbp_multiplayer_pawn) (Variables|Default|GetDamage)))
      (:CastFailed
        (Utilities|Casting|CastToBP_Projectile OtherActor
          (:CastFailed
            _))))
    (CallFunction|MilticastHitEffects Location)
    (CallFunction|ServerLIfeEnded)
    (Variables|Default|SetbCollided true)))

(event EventBeginPlay
  ;[1 1 1] Destroy On Time
  (Utilities|Time|SetTimerbyEvent (delegate Custom|Life%20Ended) (Variables|Default|GetTTL)))

(event EventTick
  (params (DeltaSeconds :type Float%20%28single-precision%29))
  ;[1 1 1] Projectile Move(Move event calls out)
  (if (Networking|IsServer)
    (CallFunction|ServerMove DeltaSeconds)))

(fn ConstructionScript)